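; Chat game mode for a turn-based game that generates a set of unique server numbers at start and relays client messages to every player.
; AnnounceTurn broadcasts Korean notices for the first, second and last turns and resets each BP_Controller's finished flag.
; CheckTurn advances the turn counter once all controllers have finished, and broadcasts a draw when the counter has reached its limit.
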(event Custom|GotMessageFromClient
  (params (Msg :type String))
  (bind _outactors (Actor|GetAllActorsOfClass "/Script/Engine.PlayerController"))
  (for _array_element _outactors
    (bind _asbp_controller (Utilities|Casting|CastToBP_Controller _array_element))
    (Default|GotBroadcast _asbp_controller Msg)))

(event Custom|CheckTurn
  (CallFunction|CheckTurnFinish)
  (if (not (Variables|Default|GetNotFinished))
    (if (< (Variables|Default|GetTurnCount) 3)
      (bind _output_get (Variables|Default|SetTurnCount (+ (Variables|Default|GetTurnCount) 1)))
      (CallFunction|AnnounceTurn _output_get)
      (else
        (bind _outactors (Actor|GetAllActorsOfClass "/Script/Engine.PlayerController"))
        (for _array_element _outactors
          (bind _asbp_controller (Utilities|Casting|CastToBP_Controller _array_element))
          (Default|GotBroadcast _asbp_controller "무승부 입니다."))))))

(event EventBeginPlay
  (bind _returnvalue (Class|RandomNumberLibrary|GenerateUniqueNumbers))
  (Variables|Default|SetServerNums _returnvalue)
  (CallFunction|AnnounceTurn (Variables|Default|GetTurnCount)))

(fn ConstructionScript)

(fn CheckTurnFinish
  (Variables|Default|SetNotFinished false)
  (bind _outactors (Actor|GetAllActorsOfClass "/Script/Engine.PlayerController"))
  (for _array_element _outactors
    (bind _asbp_controller (Utilities|Casting|CastToBP_Controller _array_element))
    (if (not (Variables|/Game/Blueprints/BP_Controller.BP_Controller_C|GetIsFinished _asbp_controller))
      (Variables|Default|SetNotFinished true))))

(fn AnnounceTurn
  (params (TurnCount :type Integer))
  (switch int TurnCount
    (:0
      (LocalVariables|SetAnswer%20Text "첫 번째 턴입니다."))
    (:1
      (LocalVariables|SetAnswer%20Text "두 번째 턴입니다."))
    (:2
      (LocalVariables|SetAnswer%20Text "마지막 턴 입니다.")))
  (bind _outactors (Actor|GetAllActorsOfClass "/Script/Engine.PlayerController"))
  (for _array_element _outactors
    (bind _asbp_controller (Utilities|Casting|CastToBP_Controller _array_element))
    (Variables|/Game/Blueprints/BP_Controller.BP_Controller_C|SetIsFinished _asbp_controller false)
    (Default|GotBroadcast _asbp_controller (LocalVariables|GetAnswer%20Text))))